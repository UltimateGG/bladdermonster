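; BP_InteractionArea is a child-actor helper that lets its parent actor be focused for player interaction.
; BeginPlay looks up parent components by "box" and "interact" tags, though the shared lookup only searches WidgetComponents and BoxRef is set to None.
; Box overlap events reset BP_FirstPersonCharacter's interaction, and CanFocus optionally requires overlap with the box.
; ToggleFocus forwards the state to the parent and shows or hides the interact widget.
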(event Custom|ToggleFocus
  (params (Focused :type Boolean))
  (bind _interactwidgetref (Variables|Default|GetInteractWidgetRef))
  (bind _output_get (Variables|Default|SetFocused Focused))
  (Class|Interactable|ToggleFocus(Message) (Actor|GetParentActor) _output_get)
  (Utilities|IsValid _interactwidgetref
    (:Is%20Valid
      (Development|SetHiddeninGame _interactwidgetref (not (Variables|Default|GetFocused)) false))))

(event Custom|OnComponentBeginOverlap_Event
  (params (OverlappedComponent :type Primitive%20Component%20Object%20Reference) (OtherActor :type Actor%20Object%20Reference) (OtherComp :type Primitive%20Component%20Object%20Reference) (OtherBodyIndex :type Integer) (bFromSweep :type Boolean) (SweepResult :type Hit%20Result%20Structure%20%28by%20ref%29))
  (bind _asbp_first_person_character (Utilities|Casting|CastToBP_FirstPersonCharacter OtherActor))
  (Default|ResetInteraction _asbp_first_person_character))

(event Custom|OnComponentEndOverlap_Event
  (params (OverlappedComponent :type Primitive%20Component%20Object%20Reference) (OtherActor :type Actor%20Object%20Reference) (OtherComp :type Primitive%20Component%20Object%20Reference) (OtherBodyIndex :type Integer))
  (bind _asbp_first_person_character (Utilities|Casting|CastToBP_FirstPersonCharacter OtherActor))
  (Default|ResetInteraction _asbp_first_person_character))

(event EventBeginPlay
  (Utilities|FlowControl|Sequence
    (:then_0
      (bind _output (CallFunction|GetTagComponent "box"))
      (Utilities|IsValid _output
        (:Is%20Valid
          (bind _output_get (Variables|Default|SetBoxRef 0))
          (Collision|AssignOnComponentBeginOverlap _output_get (delegate Custom|OnComponentBeginOverlap_Event))
          (Collision|AssignOnComponentEndOverlap (Variables|Default|GetBoxRef) (delegate Custom|OnComponentEndOverlap_Event)))))
    (:then_1
      (bind _output_2 (CallFunction|GetTagComponent "interact"))
      (Variables|Default|SetInteractWidgetRef _output_2))))

(fn ConstructionScript)

(fn CanFocus
  (params (Character :type Actor%20Object%20Reference))
  (if (Variables|Default|GetMustBeInBox)
    (return (Collision|IsOverlappingActor (Variables|Default|GetBoxRef) Character :!class /Script/Engine.PrimitiveComponent))
    (else
      (return true))))

(fn GetTagComponent
  (params (Tag :type Name))
  (bind _returnvalue (Actor|GetParentActor))
  (bind _returnvalue_2 (Actor|GetComponentsbyTag _returnvalue "/Script/UMG.WidgetComponent" Tag))
  (Utilities|IsValid _returnvalue
    (:Is%20Valid
      (if (Utilities|Array|IsNotEmpty _returnvalue_2)
        (return (Utilities|Array|Get(acopy) _returnvalue_2))))))